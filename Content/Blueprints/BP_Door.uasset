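; BP_Door is a door that slides upward when its associated pressure plate is activated with the matching key.
; On BeginPlay it binds to the plate's activated and deactivated event dispatchers.
; Activation asks the plate to check for DoorKey, then plays a timeline that lerps the door body's relative location, or prints a debug message if the key is missing.
; Deactivation reverses the same timeline to close the door.
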(event `self.ReceiveBeginPlay`
  (add `/Game/Blueprints/BP_PressurePlate.ED_PressurePlateActivated` (`self.Associated Pressure Plate`) (delegate `Door Open Signal`))
  (add `/Game/Blueprints/BP_PressurePlate.ED_PressurePlateDeactivated` (`self.Associated Pressure Plate`) (delegate `Door Close Signal`)))

(event `Door Open Signal`
  (bind _contains_key (`/Game/Blueprints/BP_PressurePlate.Check For Key ` (`self.Associated Pressure Plate`) (`self.Door Key`)))
  (if _contains_key
    (bind (_direction _door_track) (`Timeline|Door Open Timeline` :!label _label)
      (:`Update`
        (`SceneComponent.K2_SetRelativeLocation` (`self.Door Body`) (`KismetMathLibrary.VLerp` (0.0 0.0 0.0) (0.0 0.0 400.0) _door_track) false false)))
    (else
      (`KismetSystemLibrary.PrintString` "Does Not Contain Key"))))

(event `Door Close Signal`
  (goto _label :!via `Reverse`))

(fn `UserConstructionScript`)